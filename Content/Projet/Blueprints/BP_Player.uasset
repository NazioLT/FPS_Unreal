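; BP_Player is the player character Blueprint, adding run and walk speed switching on top of its parent class.
; BeginPlay calls the parent, then caches the movement component's default max walk speed as WalkSpeed.
; The Enhanced Input action IA_Run sets max walk speed to RunSpeed or the cached WalkSpeed, based on its action value on Triggered.
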(event Input|EnhancedActionEvents|EnhancedInputActionIA_Run
  (params (ActionValue :type Boolean) (ElapsedSeconds :type Float%20%28double-precision%29) (TriggeredSeconds :type Float%20%28double-precision%29) (InputAction :type Input%20Action%20Object%20Reference :default "/Game/FirstPerson/Input/Actions/IA_Run.IA_Run"))
  (:Triggered
    (Variables|/Script/Engine.CharacterMovementComponent|SetMaxWalkSpeed (Variables|Character|GetCharacterMovement) (Math|Float|SelectFloat (Variables|Default|GetRun%20Speed) (Variables|Default|GetWalk%20Speed) ActionValue))))

(event EventBeginPlay
  (|CallParentFunction)
  (Variables|Default|SetWalk%20Speed (Variables|/Script/Engine.CharacterMovementComponent|GetMaxWalkSpeed (Variables|Character|GetCharacterMovement))))

(event Collision|EventActorBeginOverlap
  (params (OtherActor :type Actor%20Object%20Reference)))

(event EventTick
  (params (DeltaSeconds :type Float%20%28single-precision%29)))

(fn ConstructionScript
  (|CallParentFunction))