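; BP_Life is a life component that tracks current health against a maximum, starting full on BeginPlay.
; Heal and Damage both route through SetLife, which clamps the value between zero and MaxLife.
; SetLife then broadcasts OnLifeUpdated with current life and percentage, and fires OnDie whenever the clamped value is zero.
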(event EventBeginPlay
  (CallFunction|SetLife (Variables|Default|GetMaxLife)))

(event EventTick
  (params (DeltaSeconds :type Float%20%28single-precision%29)))

(fn Heal
  (params (Amount :type Float%20%28double-precision%29))
  (CallFunction|SetLife (+ Amount (Variables|Default|GetCurLife))))

(fn Damage
  (params (Amount :type Float%20%28double-precision%29))
  (CallFunction|SetLife (- (Variables|Default|GetCurLife) Amount)))

(fn SetLife
  (params (Life :type Float%20%28double-precision%29))
  (bind _output_get (Variables|Default|SetCurLife (Math|Float|Clamp(Float) Life 0.0 (Variables|Default|GetMaxLife))))
  (bind _output_get_2 (Variables|Default|SetPercent (Math|Float|SafeDivide _output_get (Variables|Default|GetMaxLife))))
  (Default|CallOnLifeUpdated (Variables|Default|GetCurLife) _output_get_2)
  (if (== (Variables|Default|GetCurLife) 0.0)
    (Default|CallOnDie)))